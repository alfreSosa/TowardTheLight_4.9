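; Level game mode Blueprint that handles background music, pickup sounds and tutorial display.
; On BeginPlay it caches the LevelHUD and InfoGameInstance, adds an audio component and, if HasMusicBP passes, sets the menu track or one chosen by page name.
; Tutorial events show or hide keyed prompts on the HUD.
; Point and orb events each play their sound effect, then both call the HUD's score function.
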(event `self.ReceiveBeginPlay`
  (bind _aslevel_hud (cast `/Game/UIElementsBP/LevelHUD` (`PlayerController.GetHUD` (`GameplayStatics.GetPlayerController` null))))
  (set `self.HUD` _aslevel_hud)
  (bind _returnvalue (`AddComponent|Audio Component_1`))
  (bind _output_get (set `self.audioComponent` _returnvalue))
  (`SceneComponent.K2_SetWorldLocation` _output_get (0.0 0.0 0.0) false false)
  (bind _asinfo_game_instance (cast `InfoGameInstance` (`GameplayStatics.GetGameInstance` null)))
  (set `self.InfoGI` _asinfo_game_instance)
  (bind _returnvalue_2 (`self.HasMusicBP`))
  (if _returnvalue_2
    (`self.Play`)))

(event `self.EnterTutorialEvent`
  (params (Key :type String))
  ;[1 1 1] Tutorial
  (`/Game/UIElementsBP/LevelHUD.ShowTutorial` (`self.HUD`) Key))

(event `self.PointsSoundEvent`
  ;[1 1 1] Points
  (`GameplayStatics.PlaySoundAtLocation` null "/Game/Sounds/CoinEffect16bit.CoinEffect16bit")
  (`/Game/UIElementsBP/LevelHUD.ScoreFunc` (`self.HUD`) :!label _label))

(event `self.ExitTutorialEvent`
  (params (Key :type String))
  ;[1 1 1] Tutorial
  (`/Game/UIElementsBP/LevelHUD.HideTutorial` (`self.HUD`) Key))

(event `self.OrbsSoundEvent`
  ;[1 1 1] Orbs
  (`GameplayStatics.PlaySoundAtLocation` null "/Game/Sounds/OrbEffect16bit.OrbEffect16bit")
  (goto _label))

(fn `Play`
  (bind _audiocomponent (`self.audioComponent`))
  (bind _returnvalue (`InfoGameInstance.GetInMenu` (`self.InfoGI`)))
  (if _returnvalue
    (`AudioComponent.SetSound` _audiocomponent "/Game/Sounds/Menu_new_mix.Menu_new_mix")
    (else
      (bind _returnvalue_2 (`self.GetPageName`))
      (if (`KismetStringLibrary.EqualEqual_StrStr` _returnvalue_2 "Page1")
        (`AudioComponent.SetSound` _audiocomponent "/Game/Sounds/Track_01_Entorno_1.Track_01_Entorno_1" :!label _label)
        (elif (`KismetStringLibrary.EqualEqual_StrStr` _returnvalue_2 "Page2")
          (goto _label)
          (elif (`KismetStringLibrary.EqualEqual_StrStr` _returnvalue_2 "Page3")
            (`AudioComponent.SetSound` _audiocomponent "/Game/Sounds/Track_01_Entorno_1.Track_01_Entorno_1" :!label _label_2)
            (elif (`KismetStringLibrary.EqualEqual_StrStr` _returnvalue_2 "Page4")
              (goto _label_2)
              (else
                (`AudioComponent.SetSound` _audiocomponent "/Game/Sounds/Track_Entorno_3.Track_Entorno_3")))))))))

(fn `StopMusic`
  (`AudioComponent.Stop` (`self.audioComponent`)))

(fn `UserConstructionScript`)